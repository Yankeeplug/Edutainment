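; TranscriptAPIManagerBP sends transcript data to an HTTP API once at BeginPlay.
; It converts TranscriptData to a JSON string as the body of TranscriptUpdateRequest, then adds a hard-coded, unencrypted API key header.
; The request goes out with completion and error callbacks, which only print the response or error message.
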(event Custom|TranscriptUpdated
  (params (ResponseData :type String))
  (Development|PrintString ResponseData true true "(R=1.000000,G=0.200023,B=0.829382,A=1.000000)"))

(event Custom|TranscriptError
  (params (ErrorMessage :type String))
  (Development|PrintString ErrorMessage))

(event EventBeginPlay
  (bind _structout (Utilities|Struct|SetmembersinAIITK_NTK_JsonHttpRequestConfig (Variables|Default|GetTranscriptUpdateRequest) (Class|AIITKNTKJsonHttpFunctionLibrary|ConvertStructtoJsonString (Variables|Default|GetTranscriptData))))
  ;[0 0 0 0.5] Should probs use encrypted storage here but no one else was using it
  (Utilities|Map|Add (Utilities|Struct|BreakAIITK_NTK_JsonHttpRequestConfig _structout) "x-api-key" "sk_live_NGep5LcDfvvQeTcOXTmvDQymeF4DpbZr")
  (Class|AIITKNTKJsonHttpFunctionLibrary|SendHttpRequestwithConfig (Variables|Default|GetTranscriptUpdateRequest) (delegate Custom|TranscriptError) 0 0 (delegate Custom|TranscriptUpdated)))

(fn ConstructionScript)