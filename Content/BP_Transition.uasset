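; BP_Transition sequences a lecture level, playing its LevelParts in order as videos, GPT prompts or minigames.
; Each part creates its widget, plus a spawned GPT assistant for prompts, and binds finish events that advance to the next part.
; Minigames draw data from per-type arrays with their own counters.
; It tracks combo and streak, then shows an end screen with coins, XP and combo stats.
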(event Custom|Video%20Finished
  ;[0.15 0.15 0.15 0.5] Call part finished; check for next part.
  ;;[0.15 0.15 0.15 0.5] Downtime
  (Utilities|FlowControl|Delay 0.0)
  (CallFunction|CheckforNextPart))

(event Custom|Minigame%20Finished
  ;[0.15 0.15 0.15 0.5] Call part finished; check for next part.
  (CallFunction|AddCombo)
  (bind _returnvalue (UserInterface|CreateWidget "/Game/Widgets/WBP_GameFinished.WBP_GameFinished_C"))
  (UserInterface|Viewport|AddtoViewport _returnvalue 0)
  (Utilities|FlowControl|Delay 2.0)
  (Widget|RemovefromParent _returnvalue)
  (CallFunction|FadeOutMinigame)
  ;;[0.15 0.15 0.15 0.5] Downtime
  (Utilities|FlowControl|Delay 0.5)
  (CallFunction|RemoveMinigame)
  (CallFunction|CheckforNextPart))

(event Custom|Add%20Combo
  ;[0.15 0.15 0.15 0.5] Combo Calc
  (Math|Integer|IncrementInt (Variables|Default|GetTotal%20Combo)
    (:%20%20
      (Math|Integer|IncrementInt (Variables|Default|GetStreak)))))

(event Custom|GPT%20Finished
  ;[0.15 0.15 0.15 0.5] Call part finished; check for next part.
  (Default|FadeOut (Variables|WidgetRefs|GetCurrentPrompt))
  ;;[0.15 0.15 0.15 0.5] Downtime
  (Utilities|FlowControl|Delay 0.5)
  (Widget|RemovefromParent (Variables|WidgetRefs|GetCurrentPrompt))
  (CallFunction|CheckforNextPart))

(event Custom|Spawn%20GPT
  (params (Instructions :type String) (Prompt :type String))
  ;[0.15 0.15 0.15 0.5] Spawn BP_ResponseGPTAssistant
  (bind _returnvalue (Game|SpawnActorfromClass "/Game/Blueprints/GPT/BP_ResponseGPTAssistant.BP_ResponseGPTAssistant_C" (Math|Transform|MakeTransform "0, 0, 0") "Undefined" "MultiplyWithRoot" 0 Instructions Prompt 0))
  (Utilities|FlowControl|Delay 0.21)
  (EventDispatchers|BindEventtoGPTPartFinished (Variables|/Game/Blueprints/GPT/BP_ResponseGPTAssistant.BP_ResponseGPTAssistant_C|GetChatInterfaceWidgetRef _returnvalue) (EventDispatchers|CreateEvent :!event Custom|GPT%20Finished)))

(event Custom|Next%20Part
  (bind _level_parts (Variables|TransitionSet-up|GetLevel%20Parts))
  (bind _part_counter (Variables|Default|GetPart%20Counter))
  (bind _output (Utilities|Array|Get(acopy) _level_parts _part_counter))
  (bind (_parttype _video _audio _prompt _instructions _minigametype) (Utilities|Struct|BreakS_LectureTransition _output))
  ;[0.15 0.15 0.15 0.5] Get the information for the next lecture part.
  (Variables|Default|SetTotal%20Parts (Utilities|Array|Length _level_parts))
  (bind _returnvalue (Actor|GetActorOfClass "/Game/Blueprints/GPT/BP_ResponseGPTAssistant.BP_ResponseGPTAssistant_C"))
  (Utilities|IsValid _returnvalue
    (:Is%20Valid
      (Actor|DestroyActor _returnvalue))
    (:Is%20Not%20Valid
      _))
  (switch Utilities|FlowControl|Switch|SwitchonE_LecturePartType _parttype
    (:NewEnumerator0
      (CallFunction|AddVideo _video _audio))
    (:NewEnumerator1
      (CallFunction|AddPrompt _prompt _instructions)
      (CallFunction|SpawnGPT (Utilities|String|ToString(Text) _instructions) (Utilities|String|ToString(Text) _prompt)))
    (:NewEnumerator2
      (CallFunction|FindMinigame _minigametype))))

(event Custom|CheckForNextPart
  ;[0.15 0.15 0.15 0.5] Check to see if there is another part after this one.
  (bind _result (Math|Integer|IncrementInt (Variables|Default|GetPart%20Counter))
    (:%20%20
      (if (== _result (Variables|Default|GetTotal%20Parts))
        (CallFunction|EndOfLevelParts)
        (else
          (CallFunction|NextPart))))))

(event Custom|EndOfLevelParts
  ;[0.15 0.15 0.15 0.5] End of parts list; add the end screen with stats to viewport.
  (bind _returnvalue (UserInterface|CreateWidget "/Game/Widgets/EndRewards/WBP_LectureEndScreen.WBP_LectureEndScreen_C" (Game|GetPlayerController 0) (Variables|Rewards|GetCoins%20To%20Award) (Variables|Rewards|GetXP%20To%20Award) (Variables|Default|GetStreak) (Variables|Default|GetTotal%20Combo) (Variables|Rewards|GetDT_LecturesBase%20Row)))
  (UserInterface|Viewport|AddtoViewport _returnvalue 0))

(event Custom|Matching%20Finished
  ;[0.15 0.15 0.15 0.5] Call part finished; check for next part.
  (bind _returnvalue (UserInterface|CreateWidget "/Game/Widgets/WBP_GameFinished.WBP_GameFinished_C"))
  (UserInterface|Viewport|AddtoViewport _returnvalue 0)
  (Utilities|FlowControl|Delay 2.0)
  (Widget|RemovefromParent _returnvalue)
  (CallFunction|FadeOutMinigame)
  ;;[0.15 0.15 0.15 0.5] Downtime
  (Utilities|FlowControl|Delay 0.5)
  (CallFunction|RemoveMinigame)
  (CallFunction|CheckforNextPart))

(event Custom|Reset%20Streak
  ;[0.15 0.15 0.15 0.5] Combo Calc
  (Variables|Default|SetStreak 0))

(event EventBeginPlay
  ;[0.15 0.15 0.15 0.5] Go to first listed part.
  (CallFunction|NextPart))

(fn ConstructionScript)

(fn FindMinigame
  (params (Current%20Minigame%20Type :type E_MinigameType%20Enum :default "NewEnumerator0"))
  (switch Utilities|FlowControl|Switch|SwitchonE_MinigameType Current%20Minigame%20Type
    (:NewEnumerator0
      (CallFunction|AddSwipingCardGame))
    (:NewEnumerator1
      (CallFunction|AddMatchingCardGame))
    (:NewEnumerator2
      (CallFunction|AddCategoriesGame))
    (:NewEnumerator3
      (CallFunction|AddContradictionsGame))
    (:NewEnumerator4
      (CallFunction|AddDialogue))
    (:NewEnumerator5
      (CallFunction|AddTriviaGame))))

(fn AddPrompt
  (params (Prompt :type Text) (Instructions :type Text))
  (bind _returnvalue (UserInterface|CreateWidget "/Game/Widgets/GPT/WBP_StudentPrompt.WBP_StudentPrompt_C" (Game|GetPlayerController 0)))
  (bind _output_get (Variables|WidgetRefs|SetCurrentPrompt _returnvalue))
  (UserInterface|Viewport|AddtoViewport _output_get 0)
  (Default|Fadein _output_get)
  (Variables|/Script/UMG.TextBlock|SetText (Variables|/Game/Widgets/GPT/WBP_StudentPrompt.WBP_StudentPrompt_C|GetTxt_Instructions _output_get) Instructions)
  (Variables|/Script/UMG.TextBlock|SetText (Variables|/Game/Widgets/GPT/WBP_StudentPrompt.WBP_StudentPrompt_C|GetTxt_Prompt _output_get) Prompt))

(fn AddVideo
  (params (Video :type Media%20Source%20Object%20Reference) (Audio :type Sound%20Wave%20Object%20Reference))
  (bind _returnvalue (UserInterface|CreateWidget "/Game/Widgets/VideoPlayer/WBP_UpdatedVideoPlayer.WBP_UpdatedVideoPlayer_C" (Game|GetPlayerController 0) Video Audio))
  (UserInterface|Viewport|AddtoViewport _returnvalue 0)
  (EventDispatchers|BindEventtoVideoFinished _returnvalue (EventDispatchers|CreateEvent :!event Custom|Video%20Finished))
  (return))

(fn AddSwipingCardGame
  (bind _swipinginfo (Variables|MinigameSet-up|GetSwipingInfo))
  (bind _swipecounter (Variables|Counters|GetSwipeCounter))
  (bind _output (Utilities|Array|Get(acopy) _swipinginfo _swipecounter))
  (bind (_prompt _carddata _leftcategoryname _rightcategoryname _eventname) (Utilities|Struct|BreakS_SwipingTransitionInfo _output))
  (bind _returnvalue (UserInterface|CreateWidget "/Game/Widgets/MiniGames/SwipingMini/WBP_SwipingGame.WBP_SwipingGame_C" 0 _carddata _leftcategoryname _rightcategoryname _eventname "SwipingGameCompleted" _prompt))
  (UserInterface|Viewport|AddtoViewport _returnvalue 0)
  (bind _output_get (Variables|WidgetRefs|SetCurrentSwipingRef _returnvalue))
  (Default|Fadeon _output_get)
  (EventDispatchers|BindEventtoGameFinished _output_get (EventDispatchers|CreateEvent :!event Custom|Minigame%20Finished))
  (EventDispatchers|BindEventtoResetStreak _output_get (EventDispatchers|CreateEvent :!event Custom|Reset%20Streak))
  (Variables|Default|SetMinigameType "NewEnumerator0")
  (Math|Integer|IncrementInt (Variables|Counters|GetSwipeCounter)))

(fn AddMatchingCardGame
  (bind _matchinginfo (Variables|MinigameSet-up|GetMatchingInfo))
  (bind _matchcounter (Variables|Counters|GetMatchCounter))
  (bind _output (Utilities|Array|Get(acopy) _matchinginfo _matchcounter))
  (bind (_matchinginfo_2 _eventvalue _eventname) (Utilities|Struct|BreakS_MatchingTransitionInfo _output))
  (bind _returnvalue (UserInterface|CreateWidget "/Game/Widgets/MiniGames/MatchingMini/WBP_MatchingGame.WBP_MatchingGame_C" 0 _matchinginfo_2 _eventvalue _eventname))
  (UserInterface|Viewport|AddtoViewport _returnvalue 0)
  (bind _output_get (Variables|WidgetRefs|SetCurrentMatchingRef _returnvalue))
  (Default|Fadeon _output_get)
  (EventDispatchers|BindEventtoGameFinished _output_get (EventDispatchers|CreateEvent :!event Custom|Matching%20Finished))
  (EventDispatchers|BindEventtoResetStreak _output_get (EventDispatchers|CreateEvent :!event Custom|Reset%20Streak))
  (EventDispatchers|BindEventtoAddCombo _output_get (EventDispatchers|CreateEvent :!event Custom|Add%20Combo))
  (Variables|Default|SetMinigameType "NewEnumerator1")
  (Math|Integer|IncrementInt (Variables|Counters|GetMatchCounter)))

(fn AddCategoriesGame
  (bind _categoriesinfo (Variables|MinigameSet-up|GetCategoriesInfo))
  (bind _categorycounter (Variables|Counters|GetCategoryCounter))
  (bind _output (Utilities|Array|Get(acopy) _categoriesinfo _categorycounter))
  (bind (_prompt _categories _carddata _eventname) (Utilities|Struct|BreakS_CategoriesTransitionInfo _output))
  (bind _returnvalue (UserInterface|CreateWidget "/Game/Widgets/MiniGames/CategoriesMini/WBP_CategoriesGame.WBP_CategoriesGame_C" 0 _categories _carddata _eventname _prompt))
  (UserInterface|Viewport|AddtoViewport _returnvalue 0)
  (bind _output_get (Variables|WidgetRefs|SetCurrentCategoriesRef _returnvalue))
  (Default|Fadeon _output_get)
  (EventDispatchers|BindEventtoGameFinished _output_get (EventDispatchers|CreateEvent :!event Custom|Minigame%20Finished))
  (EventDispatchers|BindEventtoResetStreak _output_get (EventDispatchers|CreateEvent :!event Custom|Reset%20Streak))
  (Variables|Default|SetMinigameType "NewEnumerator2")
  (Math|Integer|IncrementInt (Variables|Counters|GetCategoryCounter)))

(fn AddContradictionsGame
  (bind _returnvalue (UserInterface|CreateWidget "/Game/Widgets/MiniGames/ContradictionMini/WBP_ContradictionGame.WBP_ContradictionGame_C" 0 (Utilities|Array|Get(acopy) (Variables|MinigameSet-up|GetContradictionsInfo) (Variables|Counters|GetContradictionCounter))))
  (UserInterface|Viewport|AddtoViewport _returnvalue 0)
  (bind _output_get (Variables|WidgetRefs|SetCurrentContradictionRef _returnvalue))
  (Default|Fadeon _output_get)
  (EventDispatchers|BindEventtoGameFinished _output_get (EventDispatchers|CreateEvent :!event Custom|Minigame%20Finished))
  (EventDispatchers|BindEventtoResetStreak _output_get (EventDispatchers|CreateEvent :!event Custom|Reset%20Streak))
  (Variables|Default|SetMinigameType "NewEnumerator3")
  (Math|Integer|IncrementInt (Variables|Counters|GetContradictionCounter)))

(fn AddTriviaGame
  (bind _returnvalue (UserInterface|CreateWidget "/Game/Widgets/MiniGames/TriviaUI/WBP_TriviaGame.WBP_TriviaGame_C" 0 (Utilities|Array|Get(acopy) (Variables|MinigameSet-up|GetTriviaInfo) (Variables|Counters|GetTriviaCounter))))
  (UserInterface|Viewport|AddtoViewport _returnvalue 0)
  (bind _output_get (Variables|WidgetRefs|SetCurrentTriviaRef _returnvalue))
  (EventDispatchers|BindEventtoGameFinished _output_get (EventDispatchers|CreateEvent :!event Custom|Minigame%20Finished))
  (EventDispatchers|BindEventtoResetStreak _output_get (EventDispatchers|CreateEvent :!event Custom|Reset%20Streak))
  (Variables|Default|SetMinigameType "NewEnumerator5")
  (Math|Integer|IncrementInt (Variables|Counters|GetTriviaCounter)))

(fn FadeOutMinigame
  (bind _currentswipingref (Variables|WidgetRefs|GetCurrentSwipingRef))
  (bind _currentmatchingref (Variables|WidgetRefs|GetCurrentMatchingRef))
  (bind _currentcategoriesref (Variables|WidgetRefs|GetCurrentCategoriesRef))
  (bind _currentcontradictionref (Variables|WidgetRefs|GetCurrentContradictionRef))
  (bind _currentdialogueref (Variables|WidgetRefs|GetCurrentDialogueRef))
  (switch Utilities|FlowControl|Switch|SwitchonE_MinigameType (Variables|Default|GetMinigameType)
    (:NewEnumerator0
      (Utilities|IsValid _currentswipingref
        (:Is%20Valid
          (Default|FadeOff _currentswipingref))))
    (:NewEnumerator1
      (Utilities|IsValid _currentmatchingref
        (:Is%20Valid
          (Default|FadeOff _currentmatchingref))))
    (:NewEnumerator2
      (Utilities|IsValid _currentcategoriesref
        (:Is%20Valid
          (Default|FadeOff _currentcategoriesref))))
    (:NewEnumerator3
      (Utilities|IsValid _currentcontradictionref
        (:Is%20Valid
          (Default|FadeOff _currentcontradictionref))))
    (:NewEnumerator4
      (Utilities|IsValid _currentdialogueref
        (:Is%20Valid
          (Default|FadeOff _currentdialogueref))))))

(fn RemoveMinigame
  (bind _currentswipingref (Variables|WidgetRefs|GetCurrentSwipingRef))
  (bind _currentmatchingref (Variables|WidgetRefs|GetCurrentMatchingRef))
  (bind _currentcategoriesref (Variables|WidgetRefs|GetCurrentCategoriesRef))
  (bind _currentcontradictionref (Variables|WidgetRefs|GetCurrentContradictionRef))
  (bind _currentdialogueref (Variables|WidgetRefs|GetCurrentDialogueRef))
  (switch Utilities|FlowControl|Switch|SwitchonE_MinigameType (Variables|Default|GetMinigameType)
    (:NewEnumerator0
      (Utilities|IsValid _currentswipingref
        (:Is%20Valid
          (Widget|RemovefromParent _currentswipingref))))
    (:NewEnumerator1
      (Utilities|IsValid _currentmatchingref
        (:Is%20Valid
          (Widget|RemovefromParent _currentmatchingref))))
    (:NewEnumerator2
      (Utilities|IsValid _currentcategoriesref
        (:Is%20Valid
          (Widget|RemovefromParent _currentcategoriesref))))
    (:NewEnumerator3
      (Utilities|IsValid _currentcontradictionref
        (:Is%20Valid
          (Widget|RemovefromParent _currentcontradictionref))))
    (:NewEnumerator4
      (Utilities|IsValid _currentdialogueref
        (:Is%20Valid
          (Widget|RemovefromParent _currentdialogueref))))
    (:NewEnumerator5
      (Utilities|IsValid (Variables|WidgetRefs|GetCurrentTriviaRef)
        (:Is%20Valid
          (Viewport|RemoveAllWidgets))))))

(fn AddDialogue
  (bind _returnvalue (UserInterface|CreateWidget "/Game/Widgets/MiniGames/Dialogue/WBP_DialogueDisplay.WBP_DialogueDisplay_C" 0 (Utilities|Array|Get(acopy) (Variables|MinigameSet-up|GetDialogueInfo) (Variables|Counters|GetDialogueCounter))))
  (UserInterface|Viewport|AddtoViewport _returnvalue 0)
  (bind _output_get (Variables|WidgetRefs|SetCurrentDialogueRef _returnvalue))
  (Default|Fadeon _output_get)
  (EventDispatchers|BindEventtoDialogueFinished _output_get (EventDispatchers|CreateEvent :!event Custom|Minigame%20Finished))
  (Variables|Default|SetMinigameType "NewEnumerator4")
  (Math|Integer|IncrementInt (Variables|Counters|GetDialogueCounter)))