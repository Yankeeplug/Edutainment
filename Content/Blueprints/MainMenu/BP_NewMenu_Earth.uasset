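; Earth actor for the new main menu, apparently a leftover or unfinished celestial display whose logic is mostly disconnected.
; BeginPlay plays EarthTimeline, but its update and the Tick event lead to empty sequences, and an unused lerp suggests a planned full spin.
; Unreachable branches would toggle visibility from Sun, rotational axis, ecliptic and celestial flags, alongside orphaned nodes setting a tilted or zero relative rotation.
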(event EventBeginPlay
  (Utilities|FlowControl|Sequence
    (:then_0
      (bind _newtrack_0 (Timeline|Earth%20Timeline Play)
        (:Update
          (Utilities|FlowControl|Sequence))))))

(event Collision|EventActorBeginOverlap
  (params (OtherActor :type Actor%20Object%20Reference)))

(event EventTick
  (params (DeltaSeconds :type Float%20%28single-precision%29))
  (Utilities|FlowControl|Sequence))

(fn ConstructionScript)