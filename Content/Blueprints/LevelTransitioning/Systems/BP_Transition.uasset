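; Sequencer actor that plays a lecture level's parts in order: videos, GPT prompts and minigames.
; Each part shows its widget, or for prompts also spawns a BP_ResponseGPTAssistant, then finish callbacks advance after timed downtime.
; Minigames are identified by casting to their widget class and tracked by type for fade-out and removal.
; Combo and streak counts feed the end screen along with coins and XP.
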(event Custom|Video%20Finished
  ;[0.15 0.15 0.15 0.5] Call part finished; check for next part.
  ;;[0.15 0.15 0.15 0.5] Downtime
  (Utilities|FlowControl|Delay 4.0)
  (CallFunction|CheckforNextPart))

(event Custom|Minigame%20Finished
  ;[0.15 0.15 0.15 0.5] Call part finished; check for next part.
  (CallFunction|AddCombo)
  (bind _returnvalue (UserInterface|CreateWidget "/Game/Widgets/WBP_GameFinished.WBP_GameFinished_C"))
  (UserInterface|Viewport|AddtoViewport _returnvalue 0)
  (Utilities|FlowControl|Delay 4.0)
  (Widget|RemovefromParent _returnvalue)
  (CallFunction|FadeOutMinigame)
  ;;[0.15 0.15 0.15 0.5] Downtime
  (Utilities|FlowControl|Delay 4.0)
  (CallFunction|RemoveMinigame)
  (CallFunction|CheckforNextPart))

(event Custom|Add%20Combo
  ;[0.15 0.15 0.15 0.5] Combo Calc
  (Math|Integer|IncrementInt (Variables|Default|GetTotal%20Combo)
    (:%20%20
      (Math|Integer|IncrementInt (Variables|Default|GetStreak)))))

(event Custom|GPT%20Finished
  ;[0.15 0.15 0.15 0.5] Call part finished; check for next part.
  (Default|FadeOut (Variables|Default|GetCurrentPrompt))
  ;;[0.15 0.15 0.15 0.5] Downtime
  (Utilities|FlowControl|Delay 2.0)
  (Widget|RemovefromParent (Variables|Default|GetCurrentPrompt))
  (CallFunction|CheckforNextPart))

(event Custom|Spawn%20GPT
  (params (Instructions :type String) (Prompt :type String))
  ;[0.15 0.15 0.15 0.5] Spawn BP_ResponseGPTAssistant
  (bind _returnvalue (Game|SpawnActorfromClass "/Game/Blueprints/GPT/BP_ResponseGPTAssistant.BP_ResponseGPTAssistant_C" (Math|Transform|MakeTransform "0, 0, 0") "Undefined" "MultiplyWithRoot" 0 Instructions Prompt 0))
  (Utilities|FlowControl|Delay 0.21)
  (EventDispatchers|BindEventtoGPTPartFinished (Variables|/Game/Blueprints/GPT/BP_ResponseGPTAssistant.BP_ResponseGPTAssistant_C|GetChatInterfaceWidgetRef _returnvalue) (EventDispatchers|CreateEvent :!event Custom|GPT%20Finished)))

(event Custom|Next%20Part
  (bind _level_parts (Variables|Public|GetLevel%20Parts))
  (bind _part_counter (Variables|Default|GetPart%20Counter))
  (bind _output (Utilities|Array|Get(acopy) _level_parts _part_counter))
  (bind (_parttype _video _audio _prompt _instructions _minigame) (Utilities|Struct|BreakS_LectureTransition _output))
  ;[0.15 0.15 0.15 0.5] Get the information for the next lecture part.
  (Variables|Default|SetTotal%20Parts (Utilities|Array|Length _level_parts))
  (switch Utilities|FlowControl|Switch|SwitchonE_LecturePartType _parttype
    (:NewEnumerator0
      (CallFunction|AddVideo _video _audio))
    (:NewEnumerator1
      (CallFunction|AddPrompt _prompt _instructions)
      (CallFunction|SpawnGPT (Utilities|String|ToString(Text) _instructions) (Utilities|String|ToString(Text) _prompt)))
    (:NewEnumerator2
      (CallFunction|FindMinigame _minigame))))

(event Custom|CheckForNextPart
  ;[0.15 0.15 0.15 0.5] Check to see if there is another part after this one.
  (bind _result (Math|Integer|IncrementInt (Variables|Default|GetPart%20Counter))
    (:%20%20
      (if (== _result (Variables|Default|GetTotal%20Parts))
        (CallFunction|EndOfLevelParts)
        (else
          (CallFunction|NextPart))))))

(event Custom|EndOfLevelParts
  ;[0.15 0.15 0.15 0.5] End of parts list; add the end screen with stats to viewport.
  (bind _returnvalue (UserInterface|CreateWidget "/Game/Widgets/EndRewards/WBP_LectureEndScreen.WBP_LectureEndScreen_C" (Game|GetPlayerController 0) (Variables|Public|GetCoins%20To%20Award) (Variables|Public|GetXP%20To%20Award) (Variables|Default|GetStreak) (Variables|Default|GetTotal%20Combo) (Variables|Public|GetDT_LecturesBase%20Row)))
  (UserInterface|Viewport|AddtoViewport _returnvalue 0))

(event Custom|Matching%20Finished
  ;[0.15 0.15 0.15 0.5] Call part finished; check for next part.
  (bind _returnvalue (UserInterface|CreateWidget "/Game/Widgets/WBP_GameFinished.WBP_GameFinished_C"))
  (UserInterface|Viewport|AddtoViewport _returnvalue 0)
  (Utilities|FlowControl|Delay 4.0)
  (Widget|RemovefromParent _returnvalue)
  (CallFunction|FadeOutMinigame)
  ;;[0.15 0.15 0.15 0.5] Downtime
  (Utilities|FlowControl|Delay 4.0)
  (CallFunction|RemoveMinigame)
  (CallFunction|CheckforNextPart))

(event Custom|Reset%20Streak
  ;[0.15 0.15 0.15 0.5] Combo Calc
  (Variables|Default|SetStreak 0))

(event EventBeginPlay
  ;[0.15 0.15 0.15 0.5] Go to first listed part.
  (CallFunction|NextPart))

(fn ConstructionScript)

(fn FindMinigame
  (params (Minigame :type Widget%20Object%20Reference))
  (bind _aswbp_swiping_game (Utilities|Casting|CastToWBP_SwipingGame Minigame)
    (:then
      (CallFunction|AddSwipingCardGame _aswbp_swiping_game))
    (:CastFailed
      (bind _aswbp_contradiction_game (Utilities|Casting|CastToWBP_ContradictionGame Minigame)
        (:then
          (CallFunction|AddContradictionsGame _aswbp_contradiction_game))
        (:CastFailed
          (bind _aswbp_matching_game (Utilities|Casting|CastToWBP_MatchingGame Minigame)
            (:then
              (CallFunction|AddMatchingCardGame _aswbp_matching_game))
            (:CastFailed
              (bind _aswbp_categories_game (Utilities|Casting|CastToWBP_CategoriesGame Minigame)
                (:then
                  (CallFunction|AddCategoriesGame _aswbp_categories_game))
                (:CastFailed
                  (bind _aswbp_trivia_game (Utilities|Casting|CastToWBP_TriviaGame Minigame)
                    (:then
                      (CallFunction|AddTriviaGame _aswbp_trivia_game))
                    (:CastFailed
                      (Development|PrintString "Unknown or missing minigame widget; skipping ahead to next part." true true "(R=1.000000,G=0.000177,B=0.000000,A=1.000000)" 5.0)
                      (CallFunction|CheckforNextPart))))))))))))

(fn AddPrompt
  (params (Prompt :type Text) (Instructions :type Text))
  (bind _returnvalue (UserInterface|CreateWidget "/Game/Widgets/GPT/WBP_StudentPrompt.WBP_StudentPrompt_C" (Game|GetPlayerController 0)))
  (bind _output_get (Variables|Default|SetCurrentPrompt _returnvalue))
  (UserInterface|Viewport|AddtoViewport _output_get 0)
  (Default|Fadein _output_get)
  (Variables|/Script/UMG.TextBlock|SetText (Variables|/Game/Widgets/GPT/WBP_StudentPrompt.WBP_StudentPrompt_C|GetTxt_Instructions _output_get) Instructions)
  (Variables|/Script/UMG.TextBlock|SetText (Variables|/Game/Widgets/GPT/WBP_StudentPrompt.WBP_StudentPrompt_C|GetTxt_Prompt _output_get) Prompt))

(fn AddVideo
  (params (Video :type Media%20Source%20Object%20Reference) (Audio :type Sound%20Wave%20Object%20Reference))
  (bind _returnvalue (UserInterface|CreateWidget "/Game/Widgets/VideoPlayer/WBP_UpdatedVideoPlayer.WBP_UpdatedVideoPlayer_C" (Game|GetPlayerController 0) Video Audio))
  (UserInterface|Viewport|AddtoViewport _returnvalue 0)
  (EventDispatchers|BindEventtoVideoFinished _returnvalue (EventDispatchers|CreateEvent :!event Custom|Video%20Finished))
  (return))

(fn AddSwipingCardGame
  (params (Minigame :type WBP%20Swiping%20Game%20Object%20Reference))
  (UserInterface|Viewport|AddtoViewport Minigame 0)
  (bind _output_get (Variables|MinigameRefs|SetCurrentSwipingRef Minigame))
  (Default|Fadeon _output_get)
  (EventDispatchers|BindEventtoGameFinished _output_get (EventDispatchers|CreateEvent :!event Custom|Minigame%20Finished))
  (EventDispatchers|BindEventtoResetStreak _output_get (EventDispatchers|CreateEvent :!event Custom|Reset%20Streak))
  (Variables|Default|SetMinigameType "NewEnumerator0"))

(fn AddMatchingCardGame
  (params (Minigame :type WBP%20Matching%20Game%20Object%20Reference))
  (UserInterface|Viewport|AddtoViewport Minigame 0)
  (bind _output_get (Variables|MinigameRefs|SetCurrentMatchingRef Minigame))
  (Default|Fadeon _output_get)
  (EventDispatchers|BindEventtoGameFinished _output_get (EventDispatchers|CreateEvent :!event Custom|Matching%20Finished))
  (EventDispatchers|BindEventtoResetStreak _output_get (EventDispatchers|CreateEvent :!event Custom|Reset%20Streak))
  (EventDispatchers|BindEventtoAddCombo _output_get (EventDispatchers|CreateEvent :!event Custom|Add%20Combo))
  (Variables|Default|SetMinigameType "NewEnumerator1"))

(fn AddCategoriesGame
  (params (Minigame :type WBP%20Categories%20Game%20Object%20Reference))
  (UserInterface|Viewport|AddtoViewport Minigame 0)
  (bind _output_get (Variables|MinigameRefs|SetCurrentCategoriesRef Minigame))
  (Default|Fadeon _output_get)
  (EventDispatchers|BindEventtoGameFinished _output_get (EventDispatchers|CreateEvent :!event Custom|Minigame%20Finished))
  (EventDispatchers|BindEventtoResetStreak _output_get (EventDispatchers|CreateEvent :!event Custom|Reset%20Streak))
  (Variables|Default|SetMinigameType "NewEnumerator2"))

(fn AddContradictionsGame
  (params (Minigame :type WBP%20Contradiction%20Game%20Object%20Reference))
  (UserInterface|Viewport|AddtoViewport Minigame 0)
  (bind _output_get (Variables|MinigameRefs|SetCurrentContradictionRef Minigame))
  (Default|Fadeon _output_get)
  (EventDispatchers|BindEventtoGameFinished _output_get (EventDispatchers|CreateEvent :!event Custom|Minigame%20Finished))
  (EventDispatchers|BindEventtoResetStreak _output_get (EventDispatchers|CreateEvent :!event Custom|Reset%20Streak))
  (Variables|Default|SetMinigameType "NewEnumerator3"))

(fn AddTriviaGame
  (params (CurrentMiniGameSelection :type WBP%20Trivia%20Game%20Object%20Reference))
  (UserInterface|Viewport|AddtoViewport CurrentMiniGameSelection 0)
  (bind _output_get (Variables|Default|SetCurrentTriviaRef CurrentMiniGameSelection))
  (EventDispatchers|BindEventtoGameFinished _output_get (EventDispatchers|CreateEvent :!event Custom|Minigame%20Finished))
  (EventDispatchers|BindEventtoResetStreak _output_get (EventDispatchers|CreateEvent :!event Custom|Reset%20Streak))
  (Variables|Default|SetMinigameType "NewEnumerator5"))

(fn FadeOutMinigame
  (bind _currentswipingref (Variables|MinigameRefs|GetCurrentSwipingRef))
  (bind _currentmatchingref (Variables|MinigameRefs|GetCurrentMatchingRef))
  (bind _currentcategoriesref (Variables|MinigameRefs|GetCurrentCategoriesRef))
  (bind _currentcontradictionref (Variables|MinigameRefs|GetCurrentContradictionRef))
  (bind _currentdialogueref (Variables|MinigameRefs|GetCurrentDialogueRef))
  (switch Utilities|FlowControl|Switch|SwitchonE_MinigameType (Variables|Default|GetMinigameType)
    (:NewEnumerator0
      (Utilities|IsValid _currentswipingref
        (:Is%20Valid
          (Default|FadeOff _currentswipingref))))
    (:NewEnumerator1
      (Utilities|IsValid _currentmatchingref
        (:Is%20Valid
          (Default|FadeOff _currentmatchingref))))
    (:NewEnumerator2
      (Utilities|IsValid _currentcategoriesref
        (:Is%20Valid
          (Default|FadeOff _currentcategoriesref))))
    (:NewEnumerator3
      (Utilities|IsValid _currentcontradictionref
        (:Is%20Valid
          (Default|FadeOff _currentcontradictionref))))
    (:NewEnumerator4
      (Utilities|IsValid _currentdialogueref
        (:Is%20Valid
          (Default|FadeOff _currentdialogueref))))))

(fn RemoveMinigame
  (bind _currentswipingref (Variables|MinigameRefs|GetCurrentSwipingRef))
  (bind _currentmatchingref (Variables|MinigameRefs|GetCurrentMatchingRef))
  (bind _currentcategoriesref (Variables|MinigameRefs|GetCurrentCategoriesRef))
  (bind _currentcontradictionref (Variables|MinigameRefs|GetCurrentContradictionRef))
  (bind _currentdialogueref (Variables|MinigameRefs|GetCurrentDialogueRef))
  (switch Utilities|FlowControl|Switch|SwitchonE_MinigameType (Variables|Default|GetMinigameType)
    (:NewEnumerator0
      (Utilities|IsValid _currentswipingref
        (:Is%20Valid
          (Widget|RemovefromParent _currentswipingref))))
    (:NewEnumerator1
      (Utilities|IsValid _currentmatchingref
        (:Is%20Valid
          (Widget|RemovefromParent _currentmatchingref))))
    (:NewEnumerator2
      (Utilities|IsValid _currentcategoriesref
        (:Is%20Valid
          (Widget|RemovefromParent _currentcategoriesref))))
    (:NewEnumerator3
      (Utilities|IsValid _currentcontradictionref
        (:Is%20Valid
          (Widget|RemovefromParent _currentcontradictionref))))
    (:NewEnumerator4
      (Utilities|IsValid _currentdialogueref
        (:Is%20Valid
          (Widget|RemovefromParent _currentdialogueref))))))

(fn AddDialogue
  (params (Minigame :type WBP%20Dialogue%20Display%20Object%20Reference))
  (UserInterface|Viewport|AddtoViewport Minigame 0)
  (bind _output_get (Variables|MinigameRefs|SetCurrentDialogueRef Minigame))
  (Default|Fadeon _output_get)
  (EventDispatchers|BindEventtoDialogueFinished _output_get (EventDispatchers|CreateEvent :!event Custom|Minigame%20Finished))
  (Variables|Default|SetMinigameType "NewEnumerator4"))