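; BP_Transition plays a level's intro video, then hands off to the next activity, either a minigame, a dialogue display or a GPT assistant.
; On BeginPlay it creates a video player widget from the LevelSetup video and audio and listens for its finished event.
; When playback ends, the GPTPrompt flag chooses between spawning BP_ResponseGPTAssistant and adding AfterVideoWidget to the viewport through a chain of casts to known widget types.
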(event Custom|Video%20Finished
  (if (Variables|Default|GetGPT%20Prompt?)
    (CallFunction|SpawnGPT)
    (else
      (CallFunction|FindWidget))))

(event EventBeginPlay
  (bind _level_setup (Variables|Default|GetLevel%20Setup))
  (bind (_video _audio) (Utilities|Struct|BreakS_LevelSetUp _level_setup))
  (bind _returnvalue (UserInterface|CreateWidget "/Game/Widgets/VideoPlayer/WBP_UpdatedVideoPlayer.WBP_UpdatedVideoPlayer_C" (Game|GetPlayerController 0) _video _audio))
  (Variables|Default|SetVideo%20Player _returnvalue)
  (UserInterface|Viewport|AddtoViewport _returnvalue 0)
  (EventDispatchers|BindEventtoVideoFinished _returnvalue (delegate Custom|Video%20Finished)))

(fn ConstructionScript)

(fn FindWidget
  (bind _aswbp_swiping_game (Utilities|Casting|CastToWBP_SwipingGame (Variables|Default|GetAfter%20Video%20Widget))
    (:then
      (UserInterface|Viewport|AddtoViewport _aswbp_swiping_game 0))
    (:CastFailed
      (bind _aswbp_contradiction_game (Utilities|Casting|CastToWBP_ContradictionGame (Variables|Default|GetAfter%20Video%20Widget))
        (:then
          (UserInterface|Viewport|AddtoViewport _aswbp_contradiction_game 0))
        (:CastFailed
          (bind _aswbp_matching_game (Utilities|Casting|CastToWBP_MatchingGame (Variables|Default|GetAfter%20Video%20Widget))
            (:then
              (UserInterface|Viewport|AddtoViewport _aswbp_matching_game 0))
            (:CastFailed
              (bind _aswbp_categories_game (Utilities|Casting|CastToWBP_CategoriesGame (Variables|Default|GetAfter%20Video%20Widget))
                (:then
                  (UserInterface|Viewport|AddtoViewport _aswbp_categories_game 0))
                (:CastFailed
                  (bind _aswbp_dialogue_display (Utilities|Casting|CastToWBP_DialogueDisplay (Variables|Default|GetAfter%20Video%20Widget))
                    (:then
                      (UserInterface|Viewport|AddtoViewport _aswbp_dialogue_display 0))
                    (:CastFailed
                      (Development|PrintString "After Video Widget not recognized." true true "(R=1.000000,G=0.000000,B=0.021864,A=1.000000)" 1e+01))))))))))))

(fn SpawnGPT
  (Game|SpawnActorfromClass "/Game/Blueprints/GPT/BP_ResponseGPTAssistant.BP_ResponseGPTAssistant_C" (Math|Transform|MakeTransform "0, 0, 0") "Undefined" "MultiplyWithRoot" 0 0))