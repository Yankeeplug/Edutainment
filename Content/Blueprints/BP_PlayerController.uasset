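; Player controller that adds the BGM widget and default input mapping, opens the pause menu and switches levels.
; Pause input passes through a DoOnce, creating the menu and pausing video widgets until ResetPauseCreation re-arms it.
; Left/Right arrows step an index through LevelNames, but the loop syncing it to the loaded level is disconnected.
; PlayVideo resumes only W_VideoPlayer widgets, while PauseVideo also covers W_UpdatedVideoPlayer.
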(event Custom|CurrentLevel
  (Game|GetCurrentLevelName true))

(event Custom|LoadLastLevel
  (bind _levelnames (Variables|Default|GetLevelNames))
  (CallFunction|CurrentLevel)
  (bind _output_get (Variables|Default|SetCurrent%20Level (+ (Variables|Default|GetCurrent%20Level) -1)))
  (if (Utilities|Array|IsValidIndex _levelnames _output_get)
    (Game|OpenLevel(byName) (Utilities|Array|Get(acopy) _levelnames _output_get))
    (else
      (Development|PrintString "NOT LOADING LEVEL"))))

(event Custom|LoadNextLevel
  (bind _levelnames (Variables|Default|GetLevelNames))
  (CallFunction|CurrentLevel)
  (bind _output_get (Variables|Default|SetCurrent%20Level (+ (Variables|Default|GetCurrent%20Level) 1)))
  (if (Utilities|Array|IsValidIndex _levelnames _output_get)
    (Game|OpenLevel(byName) (Utilities|Array|Get(acopy) _levelnames _output_get))
    (else
      (Development|PrintString "NOT LOADING LEVEL"))))

(event Input|EnhancedActionEvents|EnhancedInputActionIA_Pause
  (params (ActionValue :type Boolean) (ElapsedSeconds :type Float%20%28double-precision%29) (TriggeredSeconds :type Float%20%28double-precision%29) (InputAction :type Input%20Action%20Object%20Reference :default "/Game/Blueprints/Core/Inputs/IA_Pause.IA_Pause"))
  (Utilities|FlowControl|DoOnce false
    (:Completed
      (Development|PrintString "IAPAuse")
      (Utilities|FlowControl|Sequence
        (:then_0
          (bind _returnvalue (UserInterface|CreateWidget "/Game/Widgets/W_PauseMenu.W_PauseMenu_C" (Game|GetPlayerController 0)))
          (UserInterface|Viewport|AddtoViewport _returnvalue 0)
          (CallFunction|PauseVideo))))))

(event EventBeginPlay
  (Utilities|FlowControl|Sequence
    (:then_0
      (CallFunction|CurrentLevel))
    (:then_1
      (bind _returnvalue (UserInterface|CreateWidget "/Game/Widgets/MainMenu/W_BGM.W_BGM_C" (Game|GetPlayerController 0)))
      (bind _output_get (Variables|Default|SetW_BGM _returnvalue))
      (UserInterface|Viewport|AddtoViewport _output_get 1))
    (:then_2
      (bind _asbp_player_controller (Utilities|Casting|CastToBP_PlayerController (Game|GetPlayerController 0)))
      (Input|AddMappingContext (PlayerController|LocalPlayerSubsystems|GetEnhancedInputLocalPlayerSubsystem _asbp_player_controller) "/Game/Blueprints/Core/Inputs/IMC_default.IMC_default" 0 "(bIgnoreAllPressedKeysUntilRelease=True,bForceImmediately=False,bNotifyUserSettings=False)")
      (Development|PrintString "mapping context added"))))

(event EventPlayVideo
  (bind _foundwidgets (Widget|GetAllWidgetsOfClass "/Game/Widgets/VideoPlayer/W_VideoPlayer.W_VideoPlayer_C" true))
  (for _array_element _foundwidgets
    (Default|PLayVideo _array_element)))

(event EventPauseVideo
  (bind _foundwidgets (Widget|GetAllWidgetsOfClass "/Game/Widgets/VideoPlayer/W_VideoPlayer.W_VideoPlayer_C" true))
  (for _array_element _foundwidgets
    (Default|PauseVideo _array_element))
  (bind _foundwidgets_2 (Widget|GetAllWidgetsOfClass "/Game/Widgets/VideoPlayer/W_UpdatedVideoPlayer.W_UpdatedVideoPlayer_C" true))
  (for _array_element_2 _foundwidgets_2
    (Default|PauseVideo _array_element_2)))

(event EventPauseMenu
  (Utilities|FlowControl|DoOnce false
    (:Completed
      (Development|PrintString "IAPAuse")
      (Utilities|FlowControl|Sequence
        (:then_0
          (bind _returnvalue (UserInterface|CreateWidget "/Game/Widgets/W_PauseMenu.W_PauseMenu_C" (Game|GetPlayerController 0)))
          (UserInterface|Viewport|AddtoViewport _returnvalue 0)
          (CallFunction|PauseVideo))))))

(event EventResetPauseCreation
  (Utilities|FlowControl|DoOnce false) ; enters at Reset
)

(event Input|KeyboardEvents|DebugKeyT
  (params (Key :type Key%20Structure) (ActionValue :type Input%20Action%20Value%20Structure))
  (:Pressed
    (Development|PrintString "T was pressed. Here's an example of input - but we'll be using mouse and keyobard for input, mostly.")))

(event Input|KeyboardEvents|P
  (params (Key :type Key%20Structure))
  (:Pressed
    (Utilities|FlowControl|DoOnce false
      (:Completed
        (Development|PrintString "IAPAuse")
        (Utilities|FlowControl|Sequence
          (:then_0
            (bind _returnvalue (UserInterface|CreateWidget "/Game/Widgets/W_PauseMenu.W_PauseMenu_C" (Game|GetPlayerController 0)))
            (UserInterface|Viewport|AddtoViewport _returnvalue 0)
            (CallFunction|PauseVideo)))))))

(event Input|KeyboardEvents|Left
  (params (Key :type Key%20Structure))
  (:Pressed
    (CallFunction|LoadLastLevel)))

(event Input|KeyboardEvents|Right
  (params (Key :type Key%20Structure))
  (:Pressed
    (CallFunction|LoadNextLevel)))

(fn ConstructionScript)