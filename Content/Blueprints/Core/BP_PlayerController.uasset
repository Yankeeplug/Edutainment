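; Player controller for a trivia game that also sets up the BGM widget, default input mapping, UI-only input and a once-until-reset pause menu.
; AskQuestion starts a question timer and forwards to HUD_Trivia, while SetAnswer passes locked-in answers and time remaining to GS_Trivia.
; TimerExpired checks every player's PC_Trivia timer, and once none is active reveals GM_Trivia's correct answer through the HUD and prepares the next question.
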(event Custom|AskQuestion
  (params (Question :type DA%20Question%20Object%20Reference) (MultipleChoice :type Array%20of%20Texts))
  (CallFunction|StartTimer)
  (bind _ashud_trivia (Utilities|Casting|CastToHUD_Trivia (HUD|GetHUD)))
  (Default|AskQuestion _ashud_trivia Question MultipleChoice))

(event Custom|SetAnswer
  (params (Answer :type Text) (TimeRemaining :type Float%20%28double-precision%29))
  (bind _asgs_trivia (Utilities|Casting|CastToGS_Trivia (Game|GetGameState)))
  (Default|MCUpdateLockedinAnswers _asgs_trivia (Variables|GetPlayerState) Answer TimeRemaining))

(event Custom|TimerExpired
  (bind _return (CallFunction|CheckTimerStatus))
  (if _return
    (bind _asgm_trivia (Utilities|Casting|CastToGM_Trivia (Game|GetGameMode)))
    (CallFunction|CLIENTRevealAnswers (Variables|/Game/Blueprints/Minigames/Trivia_Minigame/GM_Trivia.GM_Trivia_C|GetCorrectAnswer _asgm_trivia))
    (Default|PrepareNextQuestion _asgm_trivia)))

(event Custom|CLIENT_RevealAnswers
  (params (Correct%20Answer :type Text))
  (bind _ashud_trivia (Utilities|Casting|CastToHUD_Trivia (HUD|GetHUD (Game|GetPlayerController 0))))
  (Default|RevealAnswers _ashud_trivia Correct%20Answer))

(event Input|EnhancedActionEvents|EnhancedInputActionIA_Pause
  (params (ActionValue :type Boolean) (ElapsedSeconds :type Float%20%28double-precision%29) (TriggeredSeconds :type Float%20%28double-precision%29) (InputAction :type Input%20Action%20Object%20Reference :default "/Game/Blueprints/Core/Inputs/IA_Pause.IA_Pause"))
  (Utilities|FlowControl|DoOnce false
    (:Completed
      (Development|PrintString "IAPAuse")
      (bind _returnvalue (UserInterface|CreateWidget "/Game/Widgets/WBP_PauseMenu.WBP_PauseMenu_C" (Game|GetPlayerController 0)))
      (UserInterface|Viewport|AddtoViewport _returnvalue 0)
      (CallFunction|PauseVideo))))

(event EventBeginPlay
  (Utilities|FlowControl|Sequence
    (:then_0
      (bind _returnvalue (UserInterface|CreateWidget "/Game/Widgets/MainMenu/WBP_BGM.WBP_BGM_C" (Game|GetPlayerController 0)))
      (bind _output_get (Variables|Default|SetW_BGM _returnvalue))
      (UserInterface|Viewport|AddtoViewport _output_get 1))
    (:then_1
      (bind _asbp_player_controller (Utilities|Casting|CastToBP_PlayerController (Game|GetPlayerController 0)))
      (Input|AddMappingContext (PlayerController|LocalPlayerSubsystems|GetEnhancedInputLocalPlayerSubsystem _asbp_player_controller) "/Game/Blueprints/Core/Inputs/IMC_default.IMC_default" 0 "(bIgnoreAllPressedKeysUntilRelease=True,bForceImmediately=False,bNotifyUserSettings=False)")
      (Development|PrintString "mapping context added")
      (Input|SetInputModeUIOnly self 0 "DoNotLock" false))))

(event EventPauseMenu
  (Utilities|FlowControl|DoOnce false
    (:Completed
      (Development|PrintString "IAPAuse")
      (bind _returnvalue (UserInterface|CreateWidget "/Game/Widgets/WBP_PauseMenu.WBP_PauseMenu_C" (Game|GetPlayerController 0)))
      (UserInterface|Viewport|AddtoViewport _returnvalue 0)
      (CallFunction|PauseVideo))))

(event EventResetPauseCreation
  (Utilities|FlowControl|DoOnce false) ; enters at Reset
)

(event Input|KeyboardEvents|P
  (params (Key :type Key%20Structure :default "None"))
  (:Pressed
    (Utilities|FlowControl|DoOnce false
      (:Completed
        (Development|PrintString "IAPAuse")
        (bind _returnvalue (UserInterface|CreateWidget "/Game/Widgets/WBP_PauseMenu.WBP_PauseMenu_C" (Game|GetPlayerController 0)))
        (UserInterface|Viewport|AddtoViewport _returnvalue 0)
        (CallFunction|PauseVideo)))))

(fn ConstructionScript)

(fn CheckTimerStatus
  (for _array_element (Variables|/Script/Engine.GameStateBase|GetPlayerArray (Game|GetGameState))
    (bind _aspc_trivia (Utilities|Casting|CastToPC_Trivia (Game|GetPlayerController _array_element)))
    (if (Utilities|Time|IsTimerActivebyHandle (Variables|/Game/Blueprints/Minigames/Trivia_Minigame/PC_Trivia.PC_Trivia_C|GetQuestionTimer _aspc_trivia))
      (return false)))
  (return true))

(fn StartTimer
  (bind _returnvalue (Utilities|Time|SetTimerbyEvent (EventDispatchers|CreateEvent :!event Custom|TimerExpired) 1e+01))
  (Variables|Default|SetQuestionTimer _returnvalue))