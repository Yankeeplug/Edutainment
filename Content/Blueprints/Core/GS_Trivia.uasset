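; Trivia game state that tracks each player's locked-in answer, answer time and score.
; MC_-prefixed events record or clear answers and times, announce player joins and trigger scoring, raising dispatchers for answers, joins and awarded points.
; AwardPoints loops over PlayerArray, giving correct answers a base score plus a bonus scaled by time remaining, then notifies each scoring PS_Trivia and broadcasts the new total.
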(event Custom|MC_UpdateLockedInAnswers
  (params (PlayerState :type Player%20State%20Object%20Reference) (Answer :type Text) (TimeRemaining :type Float%20%28double-precision%29))
  (Utilities|Map|Add (Variables|Default|GetLockedInAnswers) PlayerState Answer) ; What did they answer
  (Utilities|Map|Add (Variables|Default|GetPlayerTimes) PlayerState TimeRemaining) ; How quick did they answer it
  (Default|CallOnAnswerSet PlayerState Answer))

(event Custom|MC_ClearLockedInAnswers
  (Utilities|Map|Clear (Variables|Default|GetLockedInAnswers))
  (Utilities|Map|Clear (Variables|Default|GetPlayerTimes)))

(event Custom|MC_AwardPoints
  (params (CorrectAnswer :type Text))
  (CallFunction|AwardPoints CorrectAnswer))

(event Custom|MC_PlayerJoined
  (Default|CallOnPlayerJoined))

(fn ConstructionScript)

(fn AwardPoints
  (params (Correct%20Answer :type Text))
  (bind _playerscores (Variables|Default|GetPlayerScores))
  (LocalVariables|SetCorrectAnswer Correct%20Answer)
  (for _array_element (Variables|Default|GetPlayerArray)
    (bind _asps_trivia (Utilities|Casting|CastToPS_Trivia _array_element))
    (LocalVariables|SetPlayerState _asps_trivia)
    (if (Utilities|Enum|Equal(Enum) (.Value (Utilities|Map|Find (Variables|Default|GetLockedInAnswers) (LocalVariables|GetPlayerState))) (LocalVariables|GetCorrectAnswer))
      (Utilities|Map|Add _playerscores (LocalVariables|GetPlayerState) (+ (.Value (Utilities|Map|Find _playerscores (LocalVariables|GetPlayerState))) (Math|Float|Round (+ (* (.Value (Utilities|Map|Find (Variables|Default|GetPlayerTimes) (LocalVariables|GetPlayerState))) 1e+01) 1e+02))))
      (Default|OnPointsAwardedEvent (LocalVariables|GetPlayerState) (Math|Float|Round (+ (* (.Value (Utilities|Map|Find (Variables|Default|GetPlayerTimes) (LocalVariables|GetPlayerState))) 1e+01) 1e+02)))
      (Default|CallOnPointsAwarded (Math|Float|Round (+ (* (.Value (Utilities|Map|Find (Variables|Default|GetPlayerTimes) (LocalVariables|GetPlayerState))) 1e+01) 1e+02)) (+ (.Value (Utilities|Map|Find _playerscores (LocalVariables|GetPlayerState))) (Math|Float|Round (+ (* (.Value (Utilities|Map|Find (Variables|Default|GetPlayerTimes) (LocalVariables|GetPlayerState))) 1e+01) 1e+02))) (LocalVariables|GetPlayerState)))))