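; GPT vision assistant actor that sends webcam photos to GPT and shows, speaks and acts on replies.
; Media Player feeds the camera; Capture exports a render target, reloads it as a texture, and SendImage submits it as base64.
; Responses stream into the chat widget, go to ElevenLabs TTS, can trigger BSOD, color or fire via tool calls, and reveal the X button on "Prompt Completed".
; Init hardcodes both API keys.
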(event OnGPTChunkReceived(AIITKComponentBP)
  (params (Completion :type GPT%20Chat%20Completion%20Structure))
  ;[0 0 0] Responses
  (bind _responsecontent (Utilities|GetFirstChoiceContent Completion))
  (Default|UpdateLastMessageonScreen (Variables|UI|GetImageInterfaceWidgetRef) _responsecontent))

(event OnGPTCompleted(AIITKComponentBP)
  (params (Completion :type GPT%20Chat%20Completion%20Structure))
  (bind _returnvalue (Class|OpenAIFunctionLibrary|GetResponseMessage Completion))
  (bind _returnvalue_2 (Class|OpenAIFunctionLibrary|GetMessageContent _returnvalue))
  (Utilities|FlowControl|Sequence
    (:then_0
      (bind _output_get (Variables|Internal|SetCurrentChatCompletion Completion))
      (CallFunction|AddResponseMessage _output_get)
      (bind _structout (Utilities|Struct|Setmembersin11LabsRequestParams (Variables|Default|Get11LabsRequest) (Class|OpenAIFunctionLibrary|GetMessageContent (Class|OpenAIFunctionLibrary|GetResponseMessage _output_get))))
      (bind _11labsinstance (Default|SendRequestto11Labs (Variables|Default|GetAIITKComponentBP) _structout))
      (EventDispatchers|BindEventtoOnAudiowithAlignmentGenerated _11labsinstance (EventDispatchers|CreateEvent :!event AudioRecieved))
      (Utilities|RunFunctionLogic (Variables|Internal|GetCurrentChatCompletion))
      (Utilities|LogCompletion (Variables|Internal|GetCurrentChatCompletion)))
    (:then_1
      (bind _output_get_2 (Variables|Internal|SetIsCompleted (Utilities|Enum|Equal(Enum) (Utilities|String|GetSubstring _returnvalue_2 (Utilities|String|FindSubstring _returnvalue_2 "Prompt Completed" false true) 16) "Prompt Completed")))
      (if _output_get_2
        (CallFunction|PromptCompleted)))))

(event OnGPTFailed(AIITKComponentBP)
  (params (ErrorMessage :type GPT%20Chat%20Completion%20Structure))
  ;[0 0 0] Responses
  (CallFunction|AddResponseMessage ErrorMessage))

(event OnGPTModelsRetrieved(AIITKComponentBP)
  (params (ModelIds :type Array%20of%20Strings))
  ;[0 0 0] Responses
  (Default|UpdateMessagesonScreen (Variables|UI|GetImageInterfaceWidgetRef) (Utilities|ModelIdstoMessage ModelIds)))

(event 3DButtonReleased(CancelButton)
  ;[0.15 0.15 0.15 0.5] Currently has no function.  Could be added by making new buttons and custom events linked to these
)

(event 3DButtonReleased(ModelsButton)
  ;[0.15 0.15 0.15 0.5] Currently has no function.  Could be added by making new buttons and custom events linked to these
)

(event Custom|Send%20Image
  ;[0 0 0] Request
  (CallFunction|AddUserImage)
  (Default|SendRequesttoGPT (Variables|Default|GetAIITKComponentBP) (Variables|GPTOptions|GetGPTParams)))

(event Custom|GetAvaliableCameras
  (Utilities|FlowControl|Sequence
    (:then_0
      ;[0.15 0.15 0.15 0.5] Create the widget that shows user camera and allows them to take picture.
      (bind _returnvalue (UserInterface|CreateWidget "/Game/Blueprints/GPT/ImageUpload/UserCamera/W_UserCamera.W_UserCamera_C"))
      (bind _output_get (Variables|UI|SetW_UserCamera _returnvalue))
      (UserInterface|Viewport|AddtoViewport _output_get 0))
    (:then_1
      ;[0.15 0.15 0.15 0.5] Get all avaliable cameras on user device.
      (bind _outdevices (Class|MediaBlueprintFunctionLibrary|EnumerateVideoCaptureDevices (|BitmaskLiteral 15)))
      (bind _output_get_2 (Variables|Capture|SetCamera%20Devices _outdevices))
      ;[0.15 0.15 0.15 0.5] Add each camera to the dropdown box of the W_UserCamera widget
      (for _array_element _output_get_2
        (Class|ComboBoxString|AddOption (Variables|/Game/Blueprints/GPT/ImageUpload/UserCamera/W_UserCamera.W_UserCamera_C|GetCameraSelect (Variables|UI|GetW_UserCamera)) (Utilities|String|ToString(Text) (.displayname _array_element)))))))

(event Custom|Capture
  (bind _returnvalue (Class|KismetSystemLibrary|GetProjectDirectory))
  (bind _imageinterfacewidgetref (Variables|UI|GetImageInterfaceWidgetRef))
  (bind _rt_usercamera (Variables|Capture|GetRT_UserCamera))
  ;[0.15 0.15 0.15 0.5] Put camera picture onto a render target then immediately export then reload image as a Texture2D
  (Rendering|DrawMaterialtoRenderTarget _rt_usercamera (Variables|Capture|GetM_UserCamera))
  (Rendering|ExportRenderTarget _rt_usercamera _returnvalue "UserCamera")
  (Utilities|FlowControl|Delay 0.2)
  (bind _returnvalue_2 (Class|OpenAIFunctionLibrary|LoadTexturefromDisk (Utilities|String|Append _returnvalue "UserCamera")))
  (Variables|Capture|SetCurrentImage _returnvalue_2)
  ;[0.15 0.15 0.15 0.5] Bring the chat widget back
  (Default|ReturntoFocus _imageinterfacewidgetref)
  ;[0.15 0.15 0.15 0.5] Put the image on the screen
  (Appearance|SetBrushfromTexture (Variables|/Game/Blueprints/GPT/ImageUpload/W_ImageResponseGPTAssistant.W_ImageResponseGPTAssistant_C|GetPreviewImage _imageinterfacewidgetref) (Variables|Capture|GetCurrentImage) false)
  ;[0.15 0.15 0.15 0.5] Pauses the user camera (so the light turns off).
  (Sequencer|Player|Pause (Variables|Capture|GetMP_UserCamera)))

(event Custom|SwitchCamera
  (params (CameraIndex :type Integer))
  (bind _mp_usercamera (Variables|Capture|GetMP_UserCamera))
  ;[0.15 0.15 0.15 0.5] Opens the selected camera.  This is done with a Media Player.  The Media Player needs to open the URL, and needs a Media Texture to point to.
  (Utilities|FlowControl|Delay 0.2)
  (Class|MediaPlayer|OpenUrl _mp_usercamera (.url (Utilities|Array|Get(acopy) (Variables|Capture|GetCamera%20Devices) CameraIndex)))
  (Utilities|FlowControl|Delay 0.2)
  (Class|MediaPlayer|SelectTrack _mp_usercamera "Video"))

(event Custom|Activate
  ;[0.15 0.15 0.15 0.5] To be called when ready to get user input.
  (bind _returnvalue (UserInterface|CreateWidget "/Game/Blueprints/GPT/ImageUpload/W_ImageResponseGPTAssistant.W_ImageResponseGPTAssistant_C"))
  (bind _output_get (Variables|UI|SetImageInterfaceWidgetRef _returnvalue))
  (UserInterface|Viewport|AddtoViewport _output_get 0)
  (Variables|/Game/Blueprints/GPT/ImageUpload/W_ImageResponseGPTAssistant.W_ImageResponseGPTAssistant_C|SetShowSystemMessages _output_get (Variables|GPTOptions|GetShowSystemMessages)))

(event Custom|Deactivate
  ;[0.15 0.15 0.15 0.5] To be called when finished with prompt.  Might want to destroy actor as well.
  (Widget|RemovefromParent (Variables|UI|GetImageInterfaceWidgetRef)))

(event Custom|PromptCompleted
  (Widget|SetVisibility (Variables|/Game/Blueprints/GPT/ImageUpload/W_ImageResponseGPTAssistant.W_ImageResponseGPTAssistant_C|GetXButton (Variables|UI|GetImageInterfaceWidgetRef)) "Visible"))

(event EventBeginPlay
  ;[0 0 0] Init
  (|Init))

(fn ConstructionScript)

(fn AddUserImage
  (bind _returnvalue (Class|OpenAIFunctionLibrary|TexturetoBase64 (Variables|Capture|GetCurrentImage)))
  (bind _returnvalue_2 (Class|OpenAIFunctionLibrary|Base64toTexture _returnvalue))
  (Appearance|SetBrushfromTexture (Variables|/Game/Blueprints/GPT/ImageUpload/W_ImageResponseGPTAssistant.W_ImageResponseGPTAssistant_C|GetPreviewImage (Variables|UI|GetImageInterfaceWidgetRef)) _returnvalue_2 false)
  (Utilities|Array|Add (Utilities|Struct|BreakGPTChatPromptParams (Variables|GPTOptions|GetGPTParams)) (Utilities|Struct|MakeGPTChatMessage "user" (Utilities|Struct|MakeUserMessage (Utilities|Array|MakeArray (Utilities|Struct|MakeContentPart "Image" _returnvalue "")))))
  (Default|ClearUserPrompt (Variables|UI|GetImageInterfaceWidgetRef))
  (CallFunction|PlayfromSpeaker (Variables|GPTOptions|GetSendSound))
  (Default|AddNewChatObject (Variables|UI|GetImageInterfaceWidgetRef) (Utilities|Struct|MakeGPTChatMessage "assistant" "" "(Role=\"system\",Content=\"\")" "(Role=\"user\",Content=)" "(Role=\"assistant\",Content=\"\",ToolCalls=)" "(Role=\"tool\",Content=\"\",ToolCallID=\"\")" "")))

(fn AddResponseMessage
  (params (ChatCompletion :type GPT%20Chat%20Completion%20Structure%20%28by%20ref%29))
  (bind _gptparams (Variables|GPTOptions|GetGPTParams))
  (Utilities|Array|Add (Utilities|Struct|BreakGPTChatPromptParams (Variables|GPTOptions|GetGPTParams)) (Class|OpenAIFunctionLibrary|GetResponseMessage ChatCompletion))
  (Default|UpdateMessagesonScreen (Variables|UI|GetImageInterfaceWidgetRef) _gptparams)
  (Default|TruncateMessages (Variables|Default|GetAIITKComponentBP) _gptparams)
  (CallFunction|PlayfromSpeaker (Variables|GPTOptions|GetResponseSound)))

(fn PlayfromSpeaker
  (params (NewSound :type Sound%20Base%20Object%20Reference)))

(fn AddSystemMessage
  (params (Content :type String))
  (Utilities|Array|Add (.Messages (Utilities|Struct|BreakGPTChatPromptParams (Variables|GPTOptions|GetGPTParams))) (Utilities|Struct|MakeGPTChatMessage "system" "" (Utilities|Struct|MakeSystemMessage "system" Content) "(Role=\"user\",Content=)" (Utilities|Struct|MakeAssistantMessage "" 0) "(Role=\"tool\",Content=\"\",ToolCallID=\"\")" "")))

(fn AddToolResponseMessage
  (params (Tool%20Message :type Tool%20Message%20Structure))
  (bind (_role _content _toolcallid) (Utilities|Struct|BreakToolMessage Tool%20Message))
  (Utilities|Array|Add (Utilities|Struct|BreakGPTChatPromptParams (Variables|GPTOptions|GetGPTParams)) (Utilities|Struct|MakeGPTChatMessage "tool" (Utilities|Struct|MakeToolMessage _content _toolcallid))))

(fn AudioRecieved
  (params (GeneratedAudio :type Sound%20Wave%20Object%20Reference) (AlignmentData :type Character%20Alignment%20Structure%20%28by%20ref%29))
  (Audio|PlaySound2D GeneratedAudio 1.0 1.0 0.0 0 0)
  (Development|PrintString "PLAYING TTS")
  (return))